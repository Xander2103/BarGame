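; Lobby player controller that shows the lobby UI and reports the player's ready state and character choice to the game mode.
; The local controller creates W_LobbyUI with UI-only input, then requests a player info update on the server.
; Server events toggle readiness or set the selected character class.
; The class's OnRep also calls BP_LobbyGameMode's update, which only takes effect where the game mode exists, on the server.
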(event Custom|UpdatePlayerInfo
  (Utilities|FlowControl|Delay 0.1)
  (CallFunction|RunonServerUpdatePlayerInfo))

(event Custom|RunOnServerUpdatePlayerInfo
  (bind _asbp_lobby_game_mode (Utilities|Casting|CastToBP_LobbyGameMode (Game|GetGameMode)))
  (Default|UpdatePlayerInfo _asbp_lobby_game_mode self))

(event Custom|RunOnSeverToggleReadyStatus
  (bind _playerinfo (Variables|Default|GetplayerInfo))
  (Utilities|Struct|SetmembersinS_PlayerInfo _playerinfo (not (.Ready? (Utilities|Struct|BreakS_PlayerInfo _playerinfo))))
  (bind _asbp_lobby_game_mode (Utilities|Casting|CastToBP_LobbyGameMode (Game|GetGameMode)))
  (Default|UpdatePlayerInfo _asbp_lobby_game_mode self))

(event Custom|ROS_UpdateSelectedCharacter
  (params (Selected%20Character%20Class :type BP%20First%20Person%20Character%20Class%20Reference))
  (Variables|Default|SetSelected%20Character%20Class Selected%20Character%20Class))

(event EventBeginPlay
  (if (Pawn|IsLocalPlayerController)
    (bind _returnvalue (UserInterface|CreateWidget "/Game/Multiplayer/Blueprints/UI/W_LobbyUI.W_LobbyUI_C"))
    (bind _output_get (Variables|Default|SetLobbyUI _returnvalue))
    (UserInterface|Viewport|AddtoViewport _output_get 0)
    (Variables|Default|SetbShowMouseCursor true)
    (Input|SetInputModeUIOnly self (Variables|Default|GetLobbyUI) "DoNotLock" false)
    (CallFunction|RunonServerUpdatePlayerInfo)))

(fn ConstructionScript)

(fn OnRepSelectedCharacterClass
  (bind _asbp_lobby_game_mode (Utilities|Casting|CastToBP_LobbyGameMode (Game|GetGameMode)))
  (Default|UpdatePlayerInfo _asbp_lobby_game_mode self))