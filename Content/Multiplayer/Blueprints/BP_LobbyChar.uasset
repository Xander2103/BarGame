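; BP_LobbyChar is a multiplayer lobby character that displays a player's info on a widget component.
; Setting the PlayerInfo variable through updatePlayerInfo feeds its RepNotify, which passes the data to the W_PlayerInfo widget and makes the component visible.
; If the widget instance is not yet valid, the RepNotify retries itself on a short timer.
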(fn ConstructionScript)

(fn OnRepPlayerInfo
  (bind _w_playerinfo (Variables|Default|GetW_PlayerInfo))
  (bind _returnvalue (UserInterface|GetWidget _w_playerinfo))
  (Utilities|IsValid _returnvalue
    (:Is%20Valid
      (bind _asw_player_info (Utilities|Casting|CastToW_PlayerInfo _returnvalue))
      (Default|UpdatePlayerInfo _asw_player_info (Variables|Default|GetPlayerInfo))
      (Rendering|SetVisibility (Variables|Default|GetW_PlayerInfo) true false))
    (:Is%20Not%20Valid
      (Utilities|Time|SetTimerbyFunctionName 0 "OnRep_PlayerInfo" 0.1))))

(fn UpdatePlayerInfo
  (params (PlayerInfo :type S%20Player%20Info%20Structure))
  (Variables|Default|SetPlayerInfo PlayerInfo))