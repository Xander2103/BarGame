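; BP_PoolTable is the table actor for the pool minigame, caching its surface height on BeginPlay.
; When the cue ball stops overlapping the TableEdge volume, the server reports it as pocketed to the AC_PoolRules component on BP_MasterGameState.
; Completing the overview input action makes player controller 0 possess the first BP_FirstPersonCharacter found, leaving the overview camera.
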(event OnComponentEndOverlap(TableEdge)
  (params (OverlappedComponent :type Primitive%20Component%20Object%20Reference) (OtherActor :type Actor%20Object%20Reference) (OtherComp :type Primitive%20Component%20Object%20Reference) (OtherBodyIndex :type Integer))
  (Networking|SwitchHasAuthority
    (:Authority
      (bind _asbp_master_game_state (Utilities|Casting|CastToBP_MasterGameState (Game|GetGameState)))
      (bind _asbp_cue_ball (Utilities|Casting|CastToBP_CueBall OtherActor))
      (Default|ServerBallPocketed (Actor|GetComponentbyClass _asbp_master_game_state "/Game/GameRules/Pool/AC_PoolRules.AC_PoolRules_C") _asbp_cue_ball))))

(event Input|EnhancedActionEvents|EnhancedInputActionIA_SwitchToOverview
  (params (ActionValue :type Boolean) (ElapsedSeconds :type Float%20%28double-precision%29) (TriggeredSeconds :type Float%20%28double-precision%29) (InputAction :type Input%20Action%20Object%20Reference :default "/Game/Input/Actions/IA_SwitchToOverview.IA_SwitchToOverview"))
  ;[0.15 0.15 0.15 0.5] Disable Camera Overview
  (:Completed
    (bind _returnvalue (Actor|GetActorOfClass "/Game/FirstPerson/Blueprints/BP_FirstPersonCharacter.BP_FirstPersonCharacter_C"))
    (Pawn|Possess (Game|GetPlayerController 0) _returnvalue)))

(event EventBeginPlay
  (Variables|Default|SetTableSurfaceZ (.z (Transformation|GetWorldLocation (Variables|Default|GetTableSurface)))))

(event Collision|EventActorBeginOverlap
  (params (OtherActor :type Actor%20Object%20Reference)))

(event EventTick
  (params (DeltaSeconds :type Float%20%28single-precision%29)))

(fn ConstructionScript)