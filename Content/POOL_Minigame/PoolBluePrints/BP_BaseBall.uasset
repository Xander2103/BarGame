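; Base pool ball Blueprint for the pool minigame, deriving each ball's look and type from its assigned number.
; A RepNotify on BallNummer calls ApplyVisuals, which runs the lookup and sets the material on the Ball component.
; The lookup groups numbers into stripes, eight ball and solids, with indices not matching the numbers in material names.
; Stripe index 7 has no material assigned.
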(event Custom|ApplyVisuals
  (CallFunction|GetMaterial4ballNumber)
  (Rendering|Material|SetMaterial (Variables|Default|GetBall) 0 (Variables|Default|GetBallMaterial)))

(fn ConstructionScript)

(fn GetMaterial4ballNumber
  (switch int (Variables|Default|GetBallNummer)
    (:1
      ;[0.15 0.15 0.15 0.5] Stripes Needs1
      (Variables|Default|SetBallMaterial "/Game/POOL_Minigame/Textures/STRIPES/Blue10/Blue10_MTR.Blue10_MTR")
      (Variables|Default|SetBalltype "NewEnumerator2" :!label _label))
    (:2
      (Variables|Default|SetBallMaterial "/Game/POOL_Minigame/Textures/STRIPES/Brown15/Brown15_MTR.Brown15_MTR")
      (goto _label))
    (:3
      (Variables|Default|SetBallMaterial "/Game/POOL_Minigame/Textures/STRIPES/Orange13/Orange13_MTR.Orange13_MTR")
      (goto _label))
    (:4
      (Variables|Default|SetBallMaterial "/Game/POOL_Minigame/Textures/STRIPES/Purple12/Purple12_MTR.Purple12_MTR")
      (goto _label))
    (:5
      (Variables|Default|SetBallMaterial "/Game/POOL_Minigame/Textures/STRIPES/Red11/Red11_MTR.Red11_MTR")
      (goto _label))
    (:6
      (Variables|Default|SetBallMaterial "/Game/POOL_Minigame/Textures/STRIPES/Yellow9/Yellow9_MTR.Yellow9_MTR")
      (goto _label))
    (:7
      (Variables|Default|SetBallMaterial 0)
      (goto _label))
    (:8
      (Variables|Default|SetBallMaterial "/Game/POOL_Minigame/Textures/8_BALL/8_Ball_MTR.8_Ball_MTR")
      (Variables|Default|SetBalltype "NewEnumerator3"))
    (:9
      ;[0.15 0.15 0.15 0.5] Full
      (Variables|Default|SetBallMaterial "/Game/POOL_Minigame/Textures/SOLIDS/Purple4/Purple4_MTR.Purple4_MTR")
      (Variables|Default|SetBalltype "NewEnumerator1" :!label _label_2))
    (:10
      (Variables|Default|SetBallMaterial "/Game/POOL_Minigame/Textures/SOLIDS/Brown7/Brown7_MTR.Brown7_MTR")
      (goto _label_2))
    (:11
      (Variables|Default|SetBallMaterial "/Game/POOL_Minigame/Textures/SOLIDS/Red3/Red3_MTR.Red3_MTR")
      (goto _label_2))
    (:12
      (Variables|Default|SetBallMaterial "/Game/POOL_Minigame/Textures/SOLIDS/Yellow1/Yellow1_MTR.Yellow1_MTR")
      (goto _label_2))
    (:13
      (Variables|Default|SetBallMaterial "/Game/POOL_Minigame/Textures/SOLIDS/Green6/Green6_MTR.Green6_MTR")
      (goto _label_2))
    (:14
      (Variables|Default|SetBallMaterial "/Game/POOL_Minigame/Textures/SOLIDS/Orange5/Orange5_MTR.Orange5_MTR")
      (goto _label_2))
    (:15
      (Variables|Default|SetBallMaterial "/Game/POOL_Minigame/Textures/SOLIDS/Blue2/Blue2_MTR.Blue2_MTR")
      (goto _label_2))))

(fn OnRepBallNummer
  (CallFunction|ApplyVisuals))