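; Base interactable drink actor that highlights on focus through custom depth and lets a player drink it.
; Interact sets the interactor's controller as owner, then a server event passes TypeDrink to the character's ROSStartDrink and flips InteractRep.
; Its OnRep plays the drinking sound, removes the widget and child actor, and animates the mesh's Z scale by timeline before destroying it.
; Author notes flag meshes, hardcoded scale and TypeDrink as needing adjustment.
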(event Custom|InteractOnServer
  (params (interactor :type BP%20First%20Person%20Character%20Object%20Reference))
  ;[0.15 0.15 0.15 0.5] InteractDrinkingOnServer !!!!!!!!!!!!!!!!!TypeDrink Juist Zetten !!!!!!!!!!!!!!!!!!!
  (bind _asbp_first_person_player_controller (Utilities|Casting|CastToBP_FirstPersonPlayerController (Components|GetOwner)))
  (bind _asbp_first_person_character (Utilities|Casting|CastToBP_FirstPersonCharacter (Pawn|GetControlledPawn _asbp_first_person_player_controller))
    (:then
      (Development|PrintString "InteractOnServer")
      (Default|ROSStartDrink _asbp_first_person_character (Variables|Default|GetType%20Drink))
      (Variables|Default|SetinteractRep (not (Variables|Default|GetinteractRep))))
    (:CastFailed
      (Development|PrintString "fAILEDInteractOnServer"))))

(event Custom|Drink%28Anim/Audio,
  ;[0.15 0.15 0.15 0.5] Animation beer+ sound +... !!!!!!!!!!!!!!!!Meshes Altijd Aanpassen en de scale juist zetten op make vector NetQuantize!!!!!!!!!!!!!!!!!!!
  (Audio|PlaySound2D "/Game/Audio/Drinking/C_Drinking.C_Drinking" 1.0 1.0 0.0 0 0)
  (Components|DestroyComponent (Variables|Default|GetWidget))
  (Components|DestroyComponent (Variables|Default|GetChildActor))
  (bind _drink (Timeline|Timeline Play)
    (:Update
      (Transformation|SetRelativeScale3D (Variables|Default|GetStaticMesh1) (Math|Vector|MakeVectorNetQuantize 1.766261 1.766261 _drink)))
    (:Finished
      (Components|DestroyComponent (Variables|Default|GetStaticMesh1)))))

(event EventInteract
  (params (Interactor :type BP%20First%20Person%20Character%20Object%20Reference))
  ;[0.15 0.15 0.15 0.5] Interact
  (Utilities|IsValid Interactor
    (:Is%20Valid
      (Actor|SetOwner (Pawn|GetController Interactor))
      (CallFunction|InteractonServer))
    (:Is%20Not%20Valid
      (Development|PrintString "iNTERACTOR NOT VALID"))))

(event EventToggleFocus
  (params (Focus :type Boolean))
  ;[0.15 0.15 0.15 0.5] Interact
  (Utilities|IsValid (Variables|Default|GetStaticMesh1)
    (:Is%20Valid
      (Rendering|SetRenderCustomDepth (Variables|Default|GetStaticMesh) Focus))))

(fn ConstructionScript)

(fn OnRepInteractRep
  (CallFunction|Drink(Anim/Audio,))

(fn GetInteractionWidgetRef
  (return (Variables|Default|GetWidget)))