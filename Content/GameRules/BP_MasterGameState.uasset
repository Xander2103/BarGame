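; Replicated game state for a pool match, tracking turn, shot, cue ball and game-over state.
; RepNotifies for current player, turn sequence and shot-in-progress tell the first local player controller to refresh turn input.
; SetGameOver records the winner and reason on authority only.
; The cue ball notify only prints, the turn timer notify is empty, and the event graph holds unconnected debug checks.
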(fn ConstructionScript)

(fn OnRepCurrentPlayerId
  (bind _asbp_first_person_player_controller (Utilities|Casting|CastToBP_FirstPersonPlayerController (Game|GetPlayerController 0)))
  (Default|UpdateTurnInput _asbp_first_person_player_controller))

(fn OnRepTurnTimeRemaining)

(fn OnRepShotinProgress?
  (bind _asbp_first_person_player_controller (Utilities|Casting|CastToBP_FirstPersonPlayerController (Game|GetPlayerController 0)))
  (Default|UpdateTurnInput _asbp_first_person_player_controller))

(fn SetGameOver
  (params (WinnerIndex :type Integer) (Reason :type E_GameOverReason%20Enum :default "NewEnumerator0"))
  (Networking|SwitchHasAuthority
    (:Authority
      (Variables|Default|SetGameOver true)
      (Variables|Default|SetWinningPlayerIndex WinnerIndex)
      (bind _output_get (Variables|Default|SetGameOverReason Reason))
      (Development|PrintString (Utilities|String|EnumtoString _output_get)))))

(fn OnRepTurnSequence
  (bind _asbp_first_person_player_controller (Utilities|Casting|CastToBP_FirstPersonPlayerController (Game|GetPlayerController 0)))
  (Default|UpdateTurnInput _asbp_first_person_player_controller))

(fn OnRepCueBallRef
  (Development|PrintString "CueBallSpawned"))