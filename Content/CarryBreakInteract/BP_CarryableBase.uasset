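; Base replicated physics prop that players can pick up, drop, place or throw, and that shatters on hard impacts.
; Interaction runs through server events that set the carrier and notify it, while OnRep_Carrier attaches the mesh to the carrier's socket or restores physics.
; Authority-side hits pass speed, cooldown and impulse checks before multicasting sound and Niagara effects and destroying the actor.
; Focus toggles custom depth on the mesh for highlighting.
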(event OnComponentHit(Mesh)
  (params (HitComponent :type Primitive%20Component%20Object%20Reference) (OtherActor :type Actor%20Object%20Reference) (OtherComp :type Primitive%20Component%20Object%20Reference) (NormalImpulse :type Vector :default "0, 0, 0") (Hit :type Hit%20Result%20Structure%20%28by%20ref%29))
  ;[0.15 0.15 0.15 0.5] OnHitComponent
  (Networking|SwitchHasAuthority
    (:Authority
      (if (not (Variables|Default|GetIsCarried))
        (if (Utilities|IsValid (Variables|Impact|GetImpactSound))
          (bind _returnvalue (Physics|GetPhysicsLinearVelocity (Variables|Default|GetMesh) "None"))
          (if (>= (Math|Vector|VectorLength _returnvalue) (Variables|Impact|GetImpactMinSpeed))
            (if (>= (- (Utilities|Time|GetGameTimeinSeconds) (Variables|Impact|GetLastImpactTime)) (Variables|Impact|GetImpactCooldown))
              (Variables|Impact|SetLastImpactTime (Utilities|Time|GetGameTimeinSeconds))
              (if (>= (Math|Vector|VectorLength NormalImpulse) (Variables|Default|GetSchatterThreshold))
                (CallFunction|MultiCastEffects (.ImpactPoint (Collision|BreakHitResult Hit)))
                (Actor|DestroyActor)))))))))

(event Custom|Server_Throw
  (params (Interactor :type Actor%20Object%20Reference) (ThrowVelocity :type Vector))
  (CallFunction|DoThrow Interactor ThrowVelocity))

(event Custom|Server_PickUp
  (params (Interactor :type Actor%20Object%20Reference))
  ;[0.15 0.15 0.15 0.5] PickUP
  (bind _output_get (Variables|Default|SetCarrier Interactor))
  (Variables|Default|SetIsCarried true)
  (Class|Actor|SetReplicateMovement false)
  (Class|BPICarryHolder|SetCarriedActor(Message) _output_get self))

(event Custom|Server_Drop
  (params (Interactor :type Actor%20Object%20Reference))
  ;[0.15 0.15 0.15 0.5] Drop
  (if (== Interactor (Variables|Default|GetCarrier))
    (bind _output_get (Variables|Default|SetCarrier 0))
    (Development|PrintString (Utilities|GetDisplayName _output_get))
    (Variables|Default|SetIsCarried false)
    (Class|BPICarryHolder|SetCarriedActor(Message) Interactor)))

(event Custom|Server_Place
  (params (Interactor :type Actor%20Object%20Reference) (PlaceLocation :type Vector) (PlaceNormal :type Vector))
  (bind _mesh (Variables|Default|GetMesh))
  ;[0.15 0.15 0.15 0.5] Place
  (Transformation|DetachFromActor "KeepWorld" "KeepWorld" "KeepWorld")
  (Transformation|SetActorLocationAndRotation (+ PlaceLocation PlaceNormal) "0, 0, 0" false true)
  (Collision|SetCollisionEnabled _mesh "QueryAndPhysics")
  (Physics|SetSimulatePhysics _mesh true)
  (Class|Actor|SetReplicateMovement true)
  (Variables|Default|SetIsCarried false)
  (Variables|Default|SetCarrier 0)
  (Class|BPICarryHolder|SetCarriedActor(Message) Interactor))

(event Custom|DoThrow
  (params (Interactor :type Actor%20Object%20Reference) (ThrowVelocity :type Vector))
  (bind _mesh (Variables|Default|GetMesh))
  (if (and (Variables|Default|GetIsCarried) (== Interactor (Variables|Default|GetCarrier)))
    (Transformation|DetachFromActor "KeepWorld" "KeepWorld" "KeepWorld")
    (Collision|SetCollisionEnabled _mesh "QueryAndPhysics")
    (Physics|SetSimulatePhysics _mesh true)
    (Physics|SetPhysicsLinearVelocity _mesh ThrowVelocity false "None")
    (Variables|Default|SetCarrier 0)
    (Variables|Default|SetIsCarried false)
    (Class|BPICarryHolder|SetCarriedActor(Message) Interactor)))

(event Custom|MultiCast_Effects
  (params (Location :type Vector))
  (Audio|PlaySoundatLocation (Variables|Impact|GetImpactSound) Location "0, 0, 0" (Variables|Impact|GetImpactVolumeMultiplier) 1.0 0.0 "/Game/Multiplayer/SA_VoiceChat.SA_VoiceChat" 0 0 0)
  (if (Utilities|IsValid (Variables|Impact|GetImpactNiagara))
    (bind _returnvalue (Niagara|SpawnSystematLocation (Variables|Impact|GetImpactNiagara) Location "0, 0, 0" (Variables|Impact|GetImpactNiagaraScale)))
    (Variables|Default|SetNiagaraPaticle _returnvalue)))

(event EventDrop
  (params (Interactor :type Actor%20Object%20Reference))
  ;[0.15 0.15 0.15 0.5] Drop
  (Networking|SwitchHasAuthority
    (:Authority
      _)
    (:Remote
      _))
  (CallFunction|ServerDrop Interactor)
  (Development|PrintString "DropCalled"))

(event EventThrow
  (params (Ineractor :type Actor%20Object%20Reference) (ThrowVelocity :type Vector :default "0, 0, 0"))
  (Networking|SwitchHasAuthority
    (:Authority
      (CallFunction|DoThrow Ineractor ThrowVelocity))
    (:Remote
      (CallFunction|ServerThrow Ineractor ThrowVelocity))))

(event EventInteract
  (params (Interactor :type BP%20First%20Person%20Character%20Object%20Reference))
  (Actor|SetOwner Interactor)
  (if (and (Variables|Default|GetIsCarried) (== Interactor (Variables|Default|GetCarrier)))
    (CallFunction|Drop Interactor)
    (else
      (bind _returnvalue (CallFunction|CanPickUp Interactor))
      (if _returnvalue
        (CallFunction|PickUp Interactor)))))

(event EventToggleFocus
  (params (Focus :type Boolean))
  (Rendering|SetRenderCustomDepth (Variables|Default|GetMesh) Focus))

(event EventPlace
  (params (Interactor :type Actor%20Object%20Reference) (PlaceLocation :type Vector :default "0, 0, 0") (PlaceNormal :type Vector :default "0, 0, 0"))
  ;[0.15 0.15 0.15 0.5] Place
  (CallFunction|ServerPlace Interactor PlaceLocation PlaceNormal))

(event EventPickUp
  (params (Interactor :type Actor%20Object%20Reference))
  ;[0.15 0.15 0.15 0.5] PickUP
  (Networking|SwitchHasAuthority
    (:Authority
      (CallFunction|ServerPickUp Interactor))))

(fn ConstructionScript)

(fn ApplyCarriedState
  (params (Interactor :type Actor%20Object%20Reference))
  (bind _mesh (Variables|Default|GetMesh))
  (Utilities|IsValid (Variables|Default|GetCarrier)
    (:Is%20Valid
      (Collision|SetCollisionEnabled _mesh "NoCollision")
      (Physics|SetSimulatePhysics _mesh false)
      (bind _scenecomponent (Class|BPICarryHolder|GetCarryAttachComponent(Message) Interactor))
      (bind _name (Class|BPICarryHolder|GetCarrySocketName(Message) Interactor))
      (Transformation|AttachComponentToComponent _scenecomponent _name "SnapToTarget" "SnapToTarget" "SnapToTarget" true))))

(fn ApplyDroppedState
  (bind _mesh (Variables|Default|GetMesh))
  (Transformation|DetachFromActor "KeepWorld" "KeepWorld" "KeepWorld")
  (Collision|SetCollisionEnabled _mesh "QueryAndPhysics")
  (Physics|SetSimulatePhysics _mesh true)
  (Class|Actor|SetReplicateMovement true)
  (Collision|SetCollisionResponsetoChannel _mesh "ECC_Pawn" "ECR_Ignore"))

(fn OnRepCarrier
  (bind _carrier (Variables|Default|GetCarrier))
  (Utilities|IsValid _carrier
    (:Is%20Valid
      (CallFunction|ApplyCarriedState _carrier))
    (:Is%20Not%20Valid
      (CallFunction|ApplyDroppedState))))

(fn OnRepIsCarried)

(fn CanPickUp
  (params (Interactor :type Actor%20Object%20Reference))
  (return (not (Variables|Default|GetIsCarried))))

(fn CanUse
  (params (Interactor :type Actor%20Object%20Reference))
  (return false))

(fn GetInteractionWidgetRef
  (return (Variables|Default|GetWidget)))