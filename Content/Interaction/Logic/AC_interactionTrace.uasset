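; Actor component for the first-person character that detects interaction areas under the camera and triggers interactions with their parent actors.
; Each tick, a visibility line trace updates the focused area and cancels held progress when focus is lost.
; Input interacts immediately or, for areas with a duration, runs a looping timer that fills the interaction widget until complete; release cancels it.
; Completion calls InteractOnServer, which messages the parent actor, then runs a test-print hook.
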(event Custom|TryToInteract
  (params (in :type Boolean))
  (if in
    (if (Variables|Default|GetIsTracingInteractionArea)
      (bind _output_get (Variables|Default|SetinteractionDuration (Variables|/Game/Interaction/Logic/InteractionArea/BP_interactionArea_Base_DontUSE.BP_interactionArea_Base_DontUSE_C|GetInteractDuration (Variables|Default|GetFocusedInteractionArea))))
      (if (> _output_get 0.0)
        (bind _ref_widget_ (Class|BPIInteraction|GetInteractionWidgetRef(Message) (Actor|GetParentActor (Variables|Default|GetFocusedInteractionArea))))
        (bind _aswb_interaction (Utilities|Casting|CastToWB_interaction (UserInterface|GetWidget _ref_widget_)))
        (Variables|Default|SetcurrentInteractionWIdgetRef _aswb_interaction)
        (bind _returnvalue (Utilities|Time|SetTimerbyEvent (delegate Custom|UpdateInteractionProgress) (Variables|Default|GetUpdateInteractionInterval) true))
        (Variables|Default|SetInteractionTimer _returnvalue)
        (else
          (CallFunction|InteractonServer (Variables|Default|GetFocusedInteractionArea) (.AsBP%20First%20Person%20Character (Utilities|Casting|CastToBP_FirstPersonCharacter (Components|GetOwner))))
          (CallFunction|RunEventAfterInteraction))))
    (else
      (CallFunction|StopInteraction))))

(event Custom|InteractOnServer
  (params (interactionArea :type BP%20Interaction%20Area%20Base%20Dont%20USE%20Object%20Reference) (Interactor :type BP%20First%20Person%20Character%20Object%20Reference))
  (Class|BPIInteraction|Interact(Message) (Actor|GetParentActor interactionArea) Interactor))

(event Custom|UpdateInteractionProgress
  (bind _output_get (Variables|Default|SetInteractionProgress (+ (Variables|Default|GetInteractionProgress) (* (/ 1.0 (Variables|Default|GetinteractionDuration)) (Variables|Default|GetUpdateInteractionInterval)))))
  (Default|SetPercent (Variables|Default|GetcurrentInteractionWIdgetRef) _output_get)
  (if (>= (Variables|Default|GetInteractionProgress) 1.0)
    (CallFunction|StopInteraction)
    (CallFunction|InteractonServer (Variables|Default|GetFocusedInteractionArea))
    (CallFunction|RunEventAfterInteraction)))

(event EventTick
  (params (DeltaSeconds :type Float%20%28single-precision%29))
  (CallFunction|Trace))

(fn Trace
  (bind _returnvalue (Game|GetPlayerCameraManager 0))
  (bind _returnvalue_2 (Transformation|GetActorLocation _returnvalue))
  (bind (_outhit _returnvalue_3) (Collision|LineTraceByChannel _returnvalue_2 (+ _returnvalue_2 (* (Math|Vector|GetForwardVector (Transformation|GetActorRotation _returnvalue)) (Variables|Default|GetLenghtOfTheTrace))) "TraceTypeQuery1" false 0 "None"))
  (if _returnvalue_3
    (if (!= (Variables|Default|GetFocusedActor) (.HitActor (Collision|BreakHitResult _outhit)))
      (Variables|Default|SetFocusedActor (.HitActor (Collision|BreakHitResult _outhit)))
      (CallFunction|TraceInteractionArea (or (== (Utilities|GetClass (.HitActor (Collision|BreakHitResult _outhit))) "/Game/Interaction/Logic/InteractionArea/BP_interactionArea_Box.BP_interactionArea_Box_C") (== (Utilities|GetClass (.HitActor (Collision|BreakHitResult _outhit))) "/Game/Interaction/Logic/InteractionArea/BP_interactionArea_CustomShape.BP_interactionArea_CustomShape_C"))))
    (else
      (CallFunction|TraceInteractionArea false))))

(fn TraceInteractionArea
  (params (Trace :type Boolean))
  (if Trace
    (if (Variables|Default|GetIsTracingInteractionArea)
      (Default|ToggleFocus (Variables|Default|GetFocusedInteractionArea) false)
      (else
        (bind _asbp_interaction_area_base_dont_use (Utilities|Casting|CastToBP_interactionArea_Base_DontUSE (Variables|Default|GetFocusedActor)))
        (bind _output_get (Variables|Default|SetFocusedInteractionArea _asbp_interaction_area_base_dont_use))
        (Default|ToggleFocus _output_get true)
        (Variables|Default|SetIsTracingInteractionArea true)))
    (elif (Variables|Default|GetIsTracingInteractionArea)
      (Variables|Default|SetIsTracingInteractionArea false)
      (Default|ToggleFocus (Variables|Default|GetFocusedInteractionArea) false)
      (Variables|Default|SetFocusedActor 0)
      (Variables|Default|SetFocusedInteractionArea 0)
      (CallFunction|StopInteraction))))

(fn StopInteraction
  (if (> (Variables|Default|GetInteractionProgress) 0.0)
    (Utilities|Time|ClearandInvalidateTimerbyHandle (Variables|Default|GetInteractionTimer))
    (Default|SetPercent (Variables|Default|GetcurrentInteractionWIdgetRef) 0.0)
    (Variables|Default|SetInteractionProgress 0.0)
    (Variables|Default|SetcurrentInteractionWIdgetRef 0)))

(fn RunEventAfterInteraction
  (bind _output_get (LocalVariables|SetparentActor (Actor|GetParentActor (Variables|Default|GetFocusedInteractionArea))))
  (if (== (Utilities|GetClass _output_get) "/Game/Interaction/Logic/BP_TestInteractionActor.BP_TestInteractionActor_C")
    (Development|PrintString "test")))