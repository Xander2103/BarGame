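; BP_TestInteractionActor is a test interactable actor whose point light is switched on and off by interaction.
; Interact calls InteractOnServer, which flips InteractToggle, and its RepNotify sets the light's visibility to match.
; Focus toggles custom depth rendering on the cube, and a getter exposes the actor's Widget as its interaction widget.
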(event Custom|InteractOnServer
  (Variables|Default|SetinteractToggle (not (Variables|Default|GetinteractToggle))))

(event EventToggleFocus
  (params (Focus :type Boolean))
  (Rendering|SetRenderCustomDepth (Variables|Default|GetCube) Focus))

(event EventInteract
  (CallFunction|InteractonServer))

(fn ConstructionScript)

(fn OnRepInteractToggle
  (if (Variables|Default|GetinteractToggle)
    (Rendering|SetVisibility (Variables|Default|GetPointLight) true false)
    (else
      (Rendering|SetVisibility (Variables|Default|GetPointLight) false false))))

(fn GetInteractionWidgetRef
  (return (Variables|Default|GetWidget)))