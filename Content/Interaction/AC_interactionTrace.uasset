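; Interaction trace component that finds and focuses the BP_interactionArea under the player's view.
; Every tick it line-traces on Visibility from player 0's camera with persistent debug drawing, toggling area focus when the hit actor changes or is lost.
; TryToInteract only reads the focused area's duration and triggers nothing yet.
; InteractOnServer sends InteractMessage to an area's parent actor but is not called here.
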(event Custom|TryToInteract
  (params (in :type Boolean))
  (bind _focusedinteractionarea (Variables|Default|GetFocusedInteractionArea))
  (if in
    (if (Variables|Default|GetIsTracingInteractionArea)
      (bind _output_get (Variables|/Game/Interaction/InteractionArea/BP_interactionArea.BP_interactionArea_C|SetInteractDuration _focusedinteractionarea (Variables|/Game/Interaction/InteractionArea/BP_interactionArea.BP_interactionArea_C|GetInteractDuration _focusedinteractionarea)))
      (if (> _output_get 0.0)
        _))))

(event Custom|InteractOnServer
  (params (interactionArea :type BP%20Interaction%20Area%20Object%20Reference))
  (Class|BPIInteraction|Interact(Message) (Actor|GetParentActor interactionArea)))

(event EventTick
  (params (DeltaSeconds :type Float%20%28single-precision%29))
  (CallFunction|Trace))

(fn Trace
  (bind _returnvalue (Game|GetPlayerCameraManager 0))
  (bind _returnvalue_2 (Transformation|GetActorLocation _returnvalue))
  (bind (_outhit _returnvalue_3) (Collision|LineTraceByChannel _returnvalue_2 (+ _returnvalue_2 (* (Math|Vector|GetForwardVector (Transformation|GetActorRotation _returnvalue)) (Variables|Default|GetLenghtOfTheTrace))) "TraceTypeQuery1" false 0 "Persistent"))
  (if _returnvalue_3
    (if (!= (Variables|Default|GetFocusedActor) (.HitActor (Collision|BreakHitResult _outhit)))
      (Variables|Default|SetFocusedActor (.HitActor (Collision|BreakHitResult _outhit)))
      (CallFunction|TraceInteractionArea (== (Utilities|GetClass (.HitActor (Collision|BreakHitResult _outhit))) "/Game/Interaction/InteractionArea/BP_interactionArea.BP_interactionArea_C")))
    (else
      (CallFunction|TraceInteractionArea false))))

(fn TraceInteractionArea
  (params (Trace :type Boolean))
  (if Trace
    (if (Variables|Default|GetIsTracingInteractionArea)
      (Default|ToggleFocus (Variables|Default|GetFocusedInteractionArea) false)
      (else
        (bind _asbp_interaction_area (Utilities|Casting|CastToBP_interactionArea (Variables|Default|GetFocusedActor)))
        (bind _output_get (Variables|Default|SetFocusedInteractionArea _asbp_interaction_area))
        (Default|ToggleFocus _output_get true)
        (Variables|Default|SetIsTracingInteractionArea true)))
    (elif (Variables|Default|GetIsTracingInteractionArea)
      (Variables|Default|SetIsTracingInteractionArea false)
      (Default|ToggleFocus (Variables|Default|GetFocusedInteractionArea) false)
      (Variables|Default|SetFocusedActor 0)
      (Variables|Default|SetFocusedInteractionArea 0))))