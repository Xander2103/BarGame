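; BP_BallPlacer is an interactable object that teleports the referenced Balls to its placer location.
; Interact calls a server event that flips InteractRep, whose OnRep triggers the arrange event; the Arranged value is ignored, so every toggle teleports.
; Focus toggles custom depth on the mesh, and a getter exposes the interaction widget.
; Gathering rack spot components is unwired, so individual spots are unused.
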(event Custom|ArangeAllBalls
  (params (Arranged :type Boolean))
  (Transformation|SetActorLocationAndRotation (Variables|Default|Getballs) (Transformation|GetWorldLocation (Variables|Default|GetballPlacerLocation)) "0, 0, 0" false true))

(event Custom|InteractOnServer
  (Variables|Default|SetinteractRep (not (Variables|Default|GetinteractRep))))

(event EventInteract
  (params (Interactor :type BP%20First%20Person%20Character%20Object%20Reference))
  (CallFunction|InteractonServer))

(event EventToggleFocus
  (params (Focus :type Boolean))
  (Rendering|SetRenderCustomDepth (Variables|Default|GetStaticMesh) Focus))

(fn ConstructionScript)

(fn OnRepInteractRep
  (CallFunction|ArangeAllBalls (Variables|Default|GetinteractRep)))

(fn GetInteractionWidgetRef
  (return (Variables|Default|GetWidget)))